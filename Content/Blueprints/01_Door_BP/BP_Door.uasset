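; BP_Door is an interactive door that the player opens and closes with the E key while standing near it.
; Box overlap with BP_ThirdPersonCharacter enables the actor's input on player controller 0, and leaving the box disables it.
; Each E press alternates through a FlipFlop between playing and reversing the DoorRotation timeline, which drives the Door component's relative yaw.
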(event `self.Box.OnComponentBeginOverlap`
  (params (OverlappedComponent :type "PrimitiveComponent Object Reference") (OtherActor :type "Actor Object Reference") (OtherComp :type "PrimitiveComponent Object Reference") (OtherBodyIndex :type Integer) (bFromSweep :type Boolean) (SweepResult :type "HitResult Structure (by ref)"))
  ;[1 1 1] To check if player has entered the Collider
  (cast `/Game/ThirdPerson/Blueprints/BP_ThirdPersonCharacter` OtherActor)
  (`self.EnableInput` (`GameplayStatics.GetPlayerController` 0)))

(event `self.Box.OnComponentEndOverlap`
  (params (OverlappedComponent :type "PrimitiveComponent Object Reference") (OtherActor :type "Actor Object Reference") (OtherComp :type "PrimitiveComponent Object Reference") (OtherBodyIndex :type Integer))
  ;[1 1 1] To check if player has exited the Collider
  (cast `/Game/ThirdPerson/Blueprints/BP_ThirdPersonCharacter` OtherActor)
  (`self.DisableInput` (`GameplayStatics.GetPlayerController` 0) null))

(event `Key|E`
  (params (Key :type "Key Structure"))
  ;[1 1 1] To make single input alternate between values using flip-flop
  (:`Pressed`
    (`/Engine/EditorBlueprintResources/StandardMacros.FlipFlop`
      (:`A`
        ;[1 1 1] To make a smooth animation-like timeline for the door
        (bind (_direction _rotationtimeline) (`Timeline|Door Rotation` :!via `PlayFromStart` :!label _label)
          (:`Update`
            ;[1 1 1] To make door rotate on command
            (`SceneComponent.K2_SetRelativeRotation` (`self.Door`) (`KismetMathLibrary.MakeRotator` 0.0 0.0 _rotationtimeline) false false))))
      (:`B`
        (goto _label :!via `ReverseFromEnd`)))))

(fn `UserConstructionScript`)