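; BP_FootballGoal is a goal actor that detects a BP_Ball entering its box trigger and resets play.
; On BeginPlay it stores the location of the referenced ball, if valid, as the spawn point.
; On overlap it plays an enlarged hit particle effect above the goal and destroys the ball.
; After a short delay it spawns an actor at the stored location, presumably a replacement ball.
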(event `self.Box.OnComponentBeginOverlap`
  (params (OverlappedComponent :type "PrimitiveComponent Object Reference") (OtherActor :type "Actor Object Reference") (OtherComp :type "PrimitiveComponent Object Reference") (OtherBodyIndex :type Integer) (bFromSweep :type Boolean) (SweepResult :type "HitResult Structure (by ref)"))
  (bind _asbp_ball (cast `/Game/Blueprints/04_Football_BP/BP_Ball` OtherActor))
  (`GameplayStatics.SpawnEmitterAtLocation` "/Game/FXVarietyPack/Particles/P_ky_hit1.P_ky_hit1" (`KismetMathLibrary.MakeVector` (.x (`self.K2_GetActorLocation`)) (.y (`self.K2_GetActorLocation`)) (+ (.z (`self.K2_GetActorLocation`)) 300.0)) (struct) (5.0 5.0 5.0))
  (`self.K2_DestroyActor` _asbp_ball)
  (`KismetSystemLibrary.Delay` 2.0)
  (`|SpawnActorFromClass` "/Game/Blueprints/04_Football_BP/BP_Ball.BP_Ball_C" (`KismetMathLibrary.MakeTransform` (`self.BallSpawnLocation`)) "Undefined" "MultiplyWithRoot" null null))

(event `self.ReceiveBeginPlay`
  (bind _ballref (`self.BallRef`))
  (`/Engine/EditorBlueprintResources/StandardMacros.IsValid` _ballref
    (:`Is Valid`
      (set `self.BallSpawnLocation` (`self.K2_GetActorLocation` _ballref)))))

(fn `UserConstructionScript`)